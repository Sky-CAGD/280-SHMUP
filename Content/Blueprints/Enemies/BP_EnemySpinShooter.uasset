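; Enemy ship that descends to mid-screen, then stops, while firing shots in a rotating eight-way spin pattern from the moment it spawns.
; ShipMovement calls the parent movement only while Z is at or above zero, and BeginPlay loops ShootProjectile every FireRate.
; Each BP_EnemyShot spawns offset along GetSetDirection(DirNum), which also sets its MoveDirection, then DirNum advances and wraps.
; GetRandomDirection is unused, despite the "random direction" comment.
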(event `self.ShipMovement`
  (bind (_returnvalue_x _returnvalue_y _returnvalue_z) (`KismetMathLibrary.BreakVector` (`self.K2_GetActorLocation`)))
  ;[0 0 0] Move Down Until Halfway Down the Screen
  (if (>= _returnvalue_z 0.0)
    (`parent.ShipMovement`)))

(event `self.ReceiveBeginPlay`
  ;[0 0 0] Shoot Repeatedly
  (`parent.ReceiveBeginPlay`)
  (`self.Shoot Projectile` :!label _label)
  (`KismetSystemLibrary.Delay` (`self.FireRate`))
  (goto _label))

(event `Shoot Projectile`
  (bind _dirnum (`self.DirNum`))
  ;[0 0 0] Shoot in Random Direction
  (bind _returnvalue (`|SpawnActorFromClass` "/Game/Blueprints/BP_EnemyShot.BP_EnemyShot_C" (`KismetMathLibrary.MakeTransform` (+ (`self.GetSetDirection` (`self.DirNum`)) (`self.K2_GetActorLocation`))) "Undefined" "MultiplyWithRoot" null null))
  (set `/Game/Blueprints/BP_BaseProjectile.Move Direction` (`self.GetSetDirection` (`self.DirNum`)) _returnvalue)
  (`/Engine/EditorBlueprintResources/StandardMacros.IncrementInt` _dirnum
    (:`  `
      (if (== _dirnum 8)
        (set `self.DirNum` 0)))))

(fn `GetRandomDirection`
  (returns (Direction :type "Vector Structure"))
  (switch `/Game/Blueprints/Enums/ShootDirections` (cast `/Game/Blueprints/Enums/ShootDirections` (`KismetMathLibrary.Conv_IntToByte` (`KismetMathLibrary.RandomInteger` 8)))
    (:`NewEnumerator0`
      (return (0.0 0.0 1.0)))
    (:`NewEnumerator1`
      (return (1.0 0.0 1.0)))
    (:`NewEnumerator2`
      (return (1.0 0.0 0.0)))
    (:`NewEnumerator3`
      (return (1.0 0.0 -1.0)))
    (:`NewEnumerator4`
      (return (0.0 0.0 -1.0)))
    (:`NewEnumerator5`
      (return (-1.0 0.0 -1.0)))
    (:`NewEnumerator6`
      (return (-1.0 0.0 0.0)))
    (:`NewEnumerator7`
      (return (-1.0 0.0 1.0)))))

(fn `GetSetDirection`
  (params (InInt :type Integer))
  (returns (Direction :type "Vector Structure"))
  (return (select `/Game/Blueprints/Enums/ShootDirections` (cast `/Game/Blueprints/Enums/ShootDirections` (`KismetMathLibrary.Conv_IntToByte` InInt)) :`NewEnumerator0` (0.0 0.0 1.0) :`NewEnumerator1` (1.0 0.0 1.0) :`NewEnumerator2` (1.0 0.0 0.0) :`NewEnumerator3` (1.0 0.0 -1.0) :`NewEnumerator4` (0.0 0.0 -1.0) :`NewEnumerator5` (-1.0 0.0 -1.0) :`NewEnumerator6` (-1.0 0.0 0.0) :`NewEnumerator7` (-1.0 0.0 1.0) :!type "Vector Structure")))

(fn `UserConstructionScript`
  (`parent.UserConstructionScript`))