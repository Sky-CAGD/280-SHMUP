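; Homing enemy ship that continuously chases the player's ship.
; On BeginPlay it runs the parent logic, then casts the player pawn to BP_PlayerShip and caches it.
; The ShipMovement event steps toward the player at constant MoveSpeed and turns to face it with a look-at rotation.
; Only the interpolated X and Z feed the new location, keeping movement on the XZ plane.
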(event `self.ReceiveBeginPlay`
  ;[0 0 0] Get Player Ship
  (`parent.ReceiveBeginPlay`)
  (bind _asbp_player_ship (cast `/Game/Blueprints/BP_PlayerShip` (`GameplayStatics.GetPlayerPawn` 0)))
  (set `self.PlayerShip` _asbp_player_ship))

(event `self.ShipMovement`
  (bind _returnvalue (`self.K2_GetActorLocation` (`self.PlayerShip`)))
  (bind _returnvalue_2 (`KismetMathLibrary.VInterpTo_Constant` (`self.K2_GetActorLocation`) _returnvalue (`self.Delta Seconds`) (`self.MoveSpeed`)))
  (bind (_returnvalue_roll _returnvalue_pitch _returnvalue_yaw) (`KismetMathLibrary.BreakRotator` (`KismetMathLibrary.FindLookAtRotation` _returnvalue_2 _returnvalue)))
  ;[0 0 0] Move and Rotate Towards Player
  (`self.K2_SetActorLocationAndRotation` (`KismetMathLibrary.MakeVector` (.x _returnvalue_2) 0.0 (.z _returnvalue_2)) (`KismetMathLibrary.MakeRotator` _returnvalue_roll _returnvalue_pitch _returnvalue_yaw)))

(fn `UserConstructionScript`
  (`parent.UserConstructionScript`))