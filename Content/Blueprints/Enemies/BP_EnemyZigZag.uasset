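; Enemy Blueprint that adds a side-to-side zigzag movement on top of its parent class, starting at BeginPlay.
; A FlipFlop alternates between the MoveRight and MoveLeft timelines, and each one restarts the cycle when it finishes.
; Each timeline update feeds its Alpha as the X direction into a swept MoveActor call, scaled by SidewaysSpeed and delta time.
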(event `self.ReceiveBeginPlay`
  (`parent.ReceiveBeginPlay`)
  (`self.StartSidewaysMove`))

(event `StartSidewaysMove`
  ;[0 0 0] Zig Zag Movement
  (`/Engine/EditorBlueprintResources/StandardMacros.FlipFlop`
    (:`A`
      (bind (_direction _alpha) (`Timeline|MoveRight` :!via `PlayFromStart`)
        (:`Update`
          (set `self.X Dir` _alpha)
          (`/Game/Blueprints/Libraries/BP_MacroLibrary.MoveActor` (`self.Delta Seconds`) (`self.SidewaysSpeed`) (`KismetMathLibrary.MakeVector` (`self.X Dir`)) true :!label _label))
        (:`Finished`
          (`self.StartSidewaysMove` :!label _label_2))))
    (:`B`
      (bind (_direction_2 _alpha_2) (`Timeline|MoveLeft` :!via `PlayFromStart`)
        (:`Update`
          (set `self.X Dir` _alpha_2)
          (goto _label))
        (:`Finished`
          (goto _label_2))))))

(fn `UserConstructionScript`
  (`parent.UserConstructionScript`))