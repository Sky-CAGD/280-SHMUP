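; Base enemy ship Blueprint that moves downward along negative Z every tick at its move speed, with sweep.
; The Damage event subtracts from Health and destroys the ship at zero, adding its score through BP_GameInstance before destroying the actor.
; Overlapping the player ship destroys both the player and the enemy, still awarding score.
; The construction script tints both meshes with EnemyColor via dynamic material instances.
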(event `self.ReceiveTick`
  (params (DeltaSeconds :type "Float (single-precision)"))
  ;[0 0 0] Get Delta Time
  (set `self.Delta Seconds` DeltaSeconds)
  (`self.ShipMovement`))

(event `ShipMovement`
  ;[0 0 0] Move Ship
  (`/Game/Blueprints/Libraries/BP_MacroLibrary.MoveActor` (`self.Delta Seconds`) (`self.MoveSpeed`) (0.0 0.0 -1.0) true true))

(event `/Game/Blueprints/Interfaces/BPI_Damageable.Damage`
  (params (Damage :type "Float (double-precision)"))
  ;[0 0 0] Damage Ship
  (bind _output_get (set `self.Health` (- (`self.Health`) Damage)))
  (if (<= _output_get 0.0)
    (`self.Destroyed`)))

(event `/Game/Blueprints/Interfaces/BPI_Damageable.Destroyed`
  ;[0 0 0] Destroy Ship
  (bind _asbp_game_instance (cast `/Game/Blueprints/BP_GameInstance` (`GameplayStatics.GetGameInstance`)))
  (`/Game/Blueprints/BP_GameInstance.AddScore` _asbp_game_instance (`self.EnemyScore`))
  (`self.K2_DestroyActor`))

(event `self.ReceiveActorBeginOverlap`
  (params (OtherActor :type "Actor Object Reference"))
  ;[0 0 0] Destroy Player Ship and Self on Overlap
  (bind _asbp_player_ship (cast `/Game/Blueprints/BP_PlayerShip` OtherActor))
  (`/Game/Blueprints/Interfaces/BPI_Damageable.Destroyed` _asbp_player_ship)
  (`self.Destroyed`))

(fn `UserConstructionScript`
  (bind _enemycolor (`self.EnemyColor`))
  ;[0 0 0] Set Enemy Color
  (`|ExecutionSequence`
    (:`then_0`
      (bind _returnvalue (`PrimitiveComponent.CreateDynamicMaterialInstance` (`self.EnemyMesh`) 0 null "None"))
      (`MaterialInstanceDynamic.SetVectorParameterValue` _returnvalue "Color" _enemycolor))
    (:`then_1`
      (bind _returnvalue_2 (`PrimitiveComponent.CreateDynamicMaterialInstance` (`self.ConeMesh`) 0 null "None"))
      (`MaterialInstanceDynamic.SetVectorParameterValue` _returnvalue_2 "Color" _enemycolor))))