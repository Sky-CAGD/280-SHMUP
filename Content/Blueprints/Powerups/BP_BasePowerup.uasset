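; Base powerup actor that drifts along negative Z until the player ship collects it.
; Tick calls MoveActor with the configured MoveSpeed to move it each frame.
; Overlapping a BP_PlayerShip passes PowerupType to the ship's CollectPowerup, then destroys the actor.
; The construction script tints both meshes with PowerupColor through dynamic material instances.
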(event `self.ReceiveTick`
  (params (DeltaSeconds :type "Float (single-precision)"))
  ;[0 0 0] Move Powerup
  (`/Game/Blueprints/Libraries/BP_MacroLibrary.MoveActor` DeltaSeconds (`self.MoveSpeed`) (0.0 0.0 -1.0)))

(event `self.ReceiveActorBeginOverlap`
  (params (OtherActor :type "Actor Object Reference"))
  ;[0 0 0] Detect when collected by player ship
  (bind _asbp_player_ship (cast `/Game/Blueprints/BP_PlayerShip` OtherActor))
  (`/Game/Blueprints/BP_PlayerShip.CollectPowerup` _asbp_player_ship (`self.PowerupType`))
  (`self.K2_DestroyActor`))

(fn `UserConstructionScript`
  (bind _powerupcolor (`self.PowerupColor`))
  ;[0 0 0] Set Enemy Color
  (`|ExecutionSequence`
    (:`then_0`
      (bind _returnvalue (`PrimitiveComponent.CreateDynamicMaterialInstance` (`self.Mesh1`) 0 null "None"))
      (`MaterialInstanceDynamic.SetVectorParameterValue` _returnvalue "Color" _powerupcolor))
    (:`then_1`
      (bind _returnvalue_2 (`PrimitiveComponent.CreateDynamicMaterialInstance` (`self.Mesh2`) 0 null "None"))
      (`MaterialInstanceDynamic.SetVectorParameterValue` _returnvalue_2 "Color" _powerupcolor))))