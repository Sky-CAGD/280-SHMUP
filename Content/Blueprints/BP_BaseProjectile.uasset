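; Base projectile actor that travels in a set direction and damages what it hits.
; Tick moves it along its normalized move direction at its configured speed.
; On overlap with an actor implementing BPI_Damageable, it sends a damage message through the interface and destroys itself.
; The construction script tints the sphere with the projectile color using a dynamic material based on M_Laser.
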(event `self.ReceiveTick`
  (params (DeltaSeconds :type "Float (single-precision)"))
  ;[0 0 0] Move Projectile
  (`/Game/Blueprints/Libraries/BP_MacroLibrary.MoveActor` DeltaSeconds (`self.Speed`) (`self.Move Direction`) false true))

(event `self.ReceiveActorBeginOverlap`
  (params (OtherActor :type "Actor Object Reference"))
  ;[0 0 0] Check for overlaps with damageable things
  (if (`KismetSystemLibrary.DoesImplementInterface` OtherActor "/Game/Blueprints/Interfaces/BPI_Damageable.BPI_Damageable_C")
    (message `/Game/Blueprints/Interfaces/BPI_Damageable.Damage` OtherActor (`self.Damage`))
    (`self.K2_DestroyActor`)))

(fn `UserConstructionScript`
  ;[0 0 0] Set Dynamic Color
  (`/Game/Blueprints/Libraries/BP_MacroLibrary.Set Dynamic Color` (`self.Sphere`) (`self.ProjectileColor`) "Color" "/Game/Materials/M_Laser.M_Laser"))