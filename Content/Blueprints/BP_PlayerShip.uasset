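; Player ship pawn that moves on the X/Z plane, fires lasers and handles damage and powerups.
; Enhanced Input drives movement and a delay-gated shot that spawns BP_Laser above the ship.
; A hit drops an active shield; otherwise, unless invincible, it costs a GameInstance life and starts timed invincibility with a Timeline-driven mesh blink.
; The Shield powerup is functional, while Big Shot and Double Shot only print messages.
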(event `self.ReceiveBeginPlay`
  ;[0 0 0] Get Player Controller
  (bind _asbp_player_controller (cast `/Game/Blueprints/BP_PlayerController` (`GameplayStatics.GetPlayerController` 0)))
  (bind _output_get (set `self.PlayerController` _asbp_player_controller))
  (bind _returnvalue (pcsubsystem `EnhancedInputLocalPlayerSubsystem` _output_get))
  ;[0 0 0] Get Player Input
  (if (`KismetSystemLibrary.IsValid` _returnvalue)
    (`EnhancedInputSubsystemInterface.AddMappingContext` _returnvalue "/Game/Inputs/InputMappingContext.InputMappingContext" 0 (struct))
    ;[0 0 0] Get Ref to Game Instance
    (bind _asbp_game_instance (cast `/Game/Blueprints/BP_GameInstance` (`GameplayStatics.GetGameInstance`)))
    (set `self.GameInstance` _asbp_game_instance)))

(event `EnhancedInput|/Game/Inputs/IA_Move`
  (params (ActionValue :type "Vector2D Structure") (ElapsedSeconds :type "Float (double-precision)") (TriggeredSeconds :type "Float (double-precision)") (InputAction :type "InputAction Object Reference" :default "/Game/Inputs/IA_Move.IA_Move"))
  ;[0 0 0] Move Player Ship
  (:`Triggered`
    (`self.AddMovementInput` (1.0 0.0 0.0) ActionValue_X)
    (`self.AddMovementInput` (0.0 0.0 1.0) ActionValue_Y)))

(event `EnhancedInput|/Game/Inputs/IA_Shoot`
  (params (ActionValue :type Boolean) (ElapsedSeconds :type "Float (double-precision)") (TriggeredSeconds :type "Float (double-precision)") (InputAction :type "InputAction Object Reference" :default "/Game/Inputs/IA_Shoot.IA_Shoot"))
  ;[0 0 0] Shooting Input
  (:`Triggered`
    (if (`self.canShoot`)
      (`self.SpawnLaser`)
      (set `self.canShoot` false)
      (`KismetSystemLibrary.Delay` (`self.FireRate`))
      (set `self.canShoot` true))))

(event `SpawnLaser`
  ;[0 0 0] Spawn Laser
  (`|SpawnActorFromClass` "/Game/Blueprints/BP_Laser.BP_Laser_C" (`KismetMathLibrary.MakeTransform` (+ (`self.K2_GetActorLocation`) (0.0 0.0 50.0))) "Undefined" "MultiplyWithRoot" null null))

(event `CollectPowerup`
  (params (PowerupType :type "/Game/Blueprints/Enums/PowerupTypes Enum" :default "NewEnumerator3"))
  ;[0 0 0] Powerup Collection/Effects
  (switch `/Game/Blueprints/Enums/PowerupTypes` PowerupType
    (:`NewEnumerator0`
      (`self.SetShieldState` true))
    (:`NewEnumerator1`
      (`KismetSystemLibrary.PrintString` "Collected Big Shot"))
    (:`NewEnumerator2`
      (`KismetSystemLibrary.PrintString` "Collected Double Shot"))))

(event `/Game/Blueprints/Interfaces/BPI_Damageable.Damage`
  (params (Damage :type "Float (double-precision)"))
  ;[0 0 0] Ship Damage/Destroyed Events
  (`self.Destroyed`))

(event `/Game/Blueprints/Interfaces/BPI_Damageable.Destroyed`
  ;[0 0 0] Ship Damage/Destroyed Events
  (if (`self.shieldActive`)
    (`self.SetShieldState` false)
    (elif (not (`self.isInvincible`))
      (`/Game/Blueprints/BP_GameInstance.LoseLife` (`self.GameInstance`))
      (`self.Start I Frames`)
      (`KismetSystemLibrary.RetriggerableDelay` (`self.invicibilityTime`))
      (`self.End I Frames`))))

(event `Start I Frames`
  ;[0 0 0] Start/End Invincibility state
  (set `self.isInvincible` true)
  (`Timeline|Blink` :!via `PlayFromStart` :!label _label
    (:`ToggleVisibility`
      (bind _isa (`/Engine/EditorBlueprintResources/StandardMacros.FlipFlop`)
        (:`A`
          _)
        (:`B`
          _))
      (`SceneComponent.SetVisibility` (`self.ShipMesh`) _isa false))))

(event `End I Frames`
  ;[0 0 0] Start/End Invincibility state
  (set `self.isInvincible` false)
  (`SceneComponent.SetVisibility` (`self.ShipMesh`) true false)
  (goto _label :!via `Stop`))

(event `SetShieldState`
  (params (Active :type Boolean))
  ;[0 0 0] Activate/Deactivate Shield
  (bind _output_get (set `self.shieldActive` Active))
  (`SceneComponent.SetVisibility` (`self.Shield`) _output_get false))

(fn `UserConstructionScript`)