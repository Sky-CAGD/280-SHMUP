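; Enemy spawner actor that spawns a randomly chosen class from its EnemiesToSpawn array.
; SpawnEnemy places each enemy at a random point on the line between LeftBound and RightBound, converted from actor-local to world space.
; A SpawnTimeline event track calls SpawnEnemy, but nothing in the graph starts that timeline.
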(event `SpawnEnemy`
  (bind _enemiestospawn (`self.EnemiesToSpawn`))
  ;[0 0 0] Spawn Random Enemy
  (`|SpawnActorFromClass` (`|GetArrayItem` _enemiestospawn (`KismetMathLibrary.RandomInteger` (`KismetArrayLibrary.Array_Length` _enemiestospawn))) (`KismetMathLibrary.MakeTransform` (`self.RandomSpawnPoint` (`self.LeftBound`) (`self.RightBound`))) "Undefined" "MultiplyWithRoot" null null))

(fn `RandomSpawnPoint`
  (params (PointA :type "Vector Structure") (PointB :type "Vector Structure"))
  (returns (ReturnValue :type "Vector Structure"))
  (bind _returnvalue (`self.GetTransform`))
  (return (`KismetMathLibrary.VLerp` (`KismetMathLibrary.TransformLocation` _returnvalue PointA) (`KismetMathLibrary.TransformLocation` _returnvalue PointB) (`KismetMathLibrary.RandomFloat`))))

(fn `UserConstructionScript`)