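; BP_Testing is a scratch actor Blueprint holding a collection of math, random, vector, transform and trace nodes, apparently for experimenting.
; Only BeginPlay does anything, printing a zero float on screen, while Tick and the construction script are empty.
; All other nodes are unwired or unused, including a Timeline, a Statue scale setter and a Math Expression combining Power, Attack, Defense and Modifier.
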(event `self.ReceiveBeginPlay`
  (`KismetSystemLibrary.PrintString` (`KismetStringLibrary.Conv_DoubleToString` 0.0) true true (struct :`R` 1.0 :`G` 0.906558 :`A` 1.0) 15.0))

(fn `UserConstructionScript`)